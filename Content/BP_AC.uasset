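; BP_AC is an actor that blinks a spotlight a limited number of times when play begins.
; BeginPlay enters a latent loop gated by a DoN node, whose Repeat variable caps the cycle count.
; Each cycle waits Frequency seconds before each of two visibility changes, set by IsEnable and then IsDisable, and feeds back into the DoN.
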(event `self.ReceiveBeginPlay`
  (bind _frequency (`self.frequency`))
  (`/Engine/EditorBlueprintResources/StandardMacros.Do N` (`self.repeat`) :!label _label
    (:`Exit`
      (`KismetSystemLibrary.Delay` _frequency)
      (`SceneComponent.SetVisibility` (`self.SpotLight`) (`self.IsEnable`) false)
      (`KismetSystemLibrary.Delay` _frequency)
      (`SceneComponent.SetVisibility` (`self.SpotLight`) (`self.IsDisable`) false)
      (goto _label))))

(fn `UserConstructionScript`)